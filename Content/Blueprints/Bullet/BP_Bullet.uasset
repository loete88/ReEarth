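; BP_Bullet is a projectile actor that damages enemies it overlaps.
; On spawn it attaches a trail particle effect to the BulletEnd point of its static mesh.
; Each tick it compares its squared distance from the player pawn against a threshold and destroys itself when too far away.
; Overlapping a BP_Enemy calls ApplyDamage with no damage amount set, and the bullet is not destroyed on hit.
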(event EventBeginPlay
  (Effects|SpawnEmitterAttached "/Game/Blueprints/Bullet/P_Bullet_Trail.P_Bullet_Trail" (Variables|Default|GetStaticMesh) "BulletEnd" "0, 0, 0" "0, 0, 0" "2.000000,2.000000,2.000000" "SnapToTarget"))

(event EventTick
  (params (DeltaSeconds :type Float%20%28single-precision%29))
  (bind _asbp_self_player (Utilities|Casting|CastToBP_SelfPlayer (Game|Player|GetPlayerPawn 0)))
  (if (> (Math|Vector|VectorLengthSquared (- (Transformation|GetActorLocation) (Transformation|GetActorLocation _asbp_self_player))) 9e+08)
    (Actor|DestroyActor)))

(event Collision|EventActorBeginOverlap
  (params (OtherActor :type Actor%20Object%20Reference))
  (bind _asbp_enemy (Utilities|Casting|CastToBP_Enemy OtherActor))
  (Game|Damage|ApplyDamage _asbp_enemy 0.0 0 0))

(fn ConstructionScript)