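; Billboard component for BP_TestTarget that computes a yaw toward the player every tick, apparently for an aim marker.
; It takes the angle between the target's forward vector and the target-to-player vector via dot product and arccosine, signed by the right-vector dot.
; That target-relative angle is applied directly as world yaw with zero pitch and roll.
; The same tick also sets world scale to zero, collapsing the component.
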(event EventTick
  (params (DeltaSeconds :type Float%20%28single-precision%29))
  (bind _asbp_test_target (Utilities|Casting|CastToBP_TestTarget (Components|GetOwner)))
  (bind _asbp_self_player (Utilities|Casting|CastToBP_SelfPlayer (Game|Player|GetPlayerPawn 0)))
  (Variables|Default|SetPlayer _asbp_self_player)
  (Variables|Default|SetTarget _asbp_test_target)
  (if (< (Math|Vector|DotProduct (Transformation|GetActorRightVector (Variables|Default|GetTarget)) (- (Transformation|GetActorLocation (Variables|Default|GetPlayer)) (Transformation|GetActorLocation (Variables|Default|GetTarget)))) 0.0)
    (bind _output_get (Variables|Default|SetYawAngle (* (Class|KismetMathLibrary|DegAcos (/ (Math|Vector|DotProduct (Transformation|GetActorForwardVector (Variables|Default|GetTarget)) (- (Transformation|GetActorLocation (Variables|Default|GetPlayer)) (Transformation|GetActorLocation (Variables|Default|GetTarget)))) (* (Math|Vector|VectorLength (- (Transformation|GetActorLocation (Variables|Default|GetPlayer)) (Transformation|GetActorLocation (Variables|Default|GetTarget)))) (Math|Vector|VectorLength (Transformation|GetActorForwardVector (Variables|Default|GetTarget)))))) -1.0)))
    (else
      (Variables|Default|SetYawAngle (Class|KismetMathLibrary|DegAcos (/ (Math|Vector|DotProduct (Transformation|GetActorForwardVector (Variables|Default|GetTarget)) (- (Transformation|GetActorLocation (Variables|Default|GetPlayer)) (Transformation|GetActorLocation (Variables|Default|GetTarget)))) (* (Math|Vector|VectorLength (- (Transformation|GetActorLocation (Variables|Default|GetPlayer)) (Transformation|GetActorLocation (Variables|Default|GetTarget)))) (Math|Vector|VectorLength (Transformation|GetActorForwardVector (Variables|Default|GetTarget)))))))))
  (Transformation|SetWorldRotation (Math|Rotator|MakeRotator 0.0 0.0 _output_get) false false)
  (Transformation|SetWorldScale3D "0, 0, 0"))