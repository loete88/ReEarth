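; BP_TestTarget is a test target actor with a billboard marker that shows whether it is being aimed at.
; The billboard starts hidden on BeginPlay, and the AimOn and AimOff functions show and hide it along with its children.
; Capsule hit and begin-overlap events print the actor and component names for debugging, with the "Overlap" and "hIT" labels swapped between them.
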(event OnComponentHit(CapsuleComponent)
  (params (HitComponent :type Primitive%20Component%20Object%20Reference) (OtherActor :type Actor%20Object%20Reference) (OtherComp :type Primitive%20Component%20Object%20Reference) (NormalImpulse :type Vector :default "0, 0, 0") (Hit :type Hit%20Result%20Structure%20%28by%20ref%29))
  (Development|PrintString (Utilities|String|Append (Utilities|GetDisplayName OtherActor) (Utilities|GetDisplayName OtherComp) " Overlap" (Utilities|GetDisplayName self))))

(event OnComponentBeginOverlap(CapsuleComponent)
  (params (OverlappedComponent :type Primitive%20Component%20Object%20Reference) (OtherActor :type Actor%20Object%20Reference) (OtherComp :type Primitive%20Component%20Object%20Reference) (OtherBodyIndex :type Integer) (bFromSweep :type Boolean) (SweepResult :type Hit%20Result%20Structure%20%28by%20ref%29))
  (Development|PrintString (Utilities|String|Append (Utilities|GetDisplayName OtherActor) (Utilities|GetDisplayName OtherComp) " hIT" (Utilities|GetDisplayName self))))

(event EventBeginPlay
  (Rendering|SetVisibility (Variables|Default|GetBP_BillBoard) false true))

(fn ConstructionScript)

(fn Aimon
  (Rendering|SetVisibility (Variables|Default|GetBP_BillBoard) true true))

(fn AimOff
  (Rendering|SetVisibility (Variables|Default|GetBP_BillBoard) false true))