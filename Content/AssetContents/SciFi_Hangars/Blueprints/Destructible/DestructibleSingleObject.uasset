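; Destructible single-object actor from the SciFi Hangars pack that breaks loose when hit.
; On Hit, a component not yet simulating physics starts simulating, unless the other component's object type is Destructible.
; Either way, each Arrow child of the Box marks an attach point for a P_Rebar particle emitter, and the hit component is set to ignore Pawn collision.
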(event EventBeginPlay)

(event Collision|EventActorBeginOverlap
  (params (OtherActor :type Actor%20Object%20Reference)))

(event EventTick
  (params (DeltaSeconds :type Float%20%28single-precision%29)))

(event Collision|EventHit
  (params (MyComp :type Primitive%20Component%20Object%20Reference) (Other :type Actor%20Object%20Reference) (OtherComp :type Primitive%20Component%20Object%20Reference) (bSelfMoved :type Boolean) (HitLocation :type Vector :default "0, 0, 0") (HitNormal :type Vector :default "0, 0, 0") (NormalImpulse :type Vector :default "0, 0, 0") (Hit :type Hit%20Result%20Structure%20%28by%20ref%29))
  (if (not (Physics|IsSimulatingPhysics MyComp "None"))
    (Physics|SetSimulatePhysics MyComp (Utilities|Enum|NotEqual(Enum) (Collision|GetCollisionObjectType OtherComp) "ECC_Destructible"))
    (for _array_element (Components|GetChildrenComponents (Variables|Default|GetBox) false)
      (bind _asarrow_component (Utilities|Casting|CastToArrowComponent _array_element))
      (Effects|SpawnEmitterAttached "/Game/AssetContents/SciFi_Hangars/Blueprints/Particle/P_Rebar.P_Rebar" _asarrow_component "None")
      (Collision|SetCollisionResponsetoChannel MyComp "ECC_Pawn" "ECR_Ignore"))))

(fn ConstructionScript)