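; Destructible sci-fi hangar lamp that flickers briefly once knocked loose, then goes permanently dark.
; Tick watches for the root mesh simulating physics, starts the flicker event and marks the lamp dead after a short delay.
; The flicker event re-calls itself through a short Delay until death, toggling a static mesh, spot light and point light via LightSet.
; Once dead, Tick keeps forcing the lights off every frame.
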(event Custom|TurnOn/Off
  ;[1 1 1] 깜빡임
  (if (Variables|Default|GetTurnLight)
    (Variables|Default|SetTurnLight false)
    (else
      (Variables|Default|SetTurnLight true)))
  (Utilities|FlowControl|Delay 0.05)
  (Utilities|LightSet (Variables|Default|GetTurnLight))
  (if (not (Variables|Default|GetisDead))
    (CallFunction|TurnOn/Off)))

(event EventTick
  (params (DeltaSeconds :type Float%20%28single-precision%29))
  (if (Variables|Default|GetisDead)
    (Utilities|LightSet false)
    (elif (Physics|IsSimulatingPhysics (Variables|Default|GetRootMesh) "None")
      (CallFunction|TurnOn/Off)
      (Utilities|FlowControl|Delay 0.5)
      (Variables|Default|SetisDead true))))

(fn ConstructionScript
  (|CallParentFunction))