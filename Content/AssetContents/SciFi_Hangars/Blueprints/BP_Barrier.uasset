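; BP_Barrier builds a straight barrier from repeated copies of a mesh, with a box sized to span the row.
; The CreateBarrier event adds static mesh components along local X, spaced by MeshSize, offset to roughly center the row and lowered on Z.
; It then scales the Box extent from BarrierSize and MeshSize, keeping depth and height fixed.
; The construction script is empty, so the barrier only appears when CreateBarrier is called.
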(event EventCreateBarrier
  (params (num :type Integer))
  (for _index (range 0 (Variables|Default|GetBarrierSize))
    (bind _returnvalue (AddComponent|AddStaticMeshComponent false (Math|Transform|MakeTransform (Math|Vector|MakeVector (- (* _index (Variables|Default|GetMeshSize)) (/ (* (+ (Variables|Default|GetBarrierSize) 1) (Variables|Default|GetMeshSize)) 2.0)) 0.0 -397.0) "0, 0, 0" "1,1,1")))
    (Components|StaticMesh|SetStaticMesh _returnvalue (Variables|Default|GetBarrierMesh)))
  (Variables|Default|SetBoxSize (/ (* (+ (Variables|Default|GetBarrierSize) 1) (Variables|Default|GetMeshSize)) 2.0))
  (Components|Box|SetBoxExtent (Variables|Default|GetBox) (Math|Vector|MakeVector (Variables|Default|GetBoxSize) 32.0 2e+03) true))

(fn ConstructionScript)