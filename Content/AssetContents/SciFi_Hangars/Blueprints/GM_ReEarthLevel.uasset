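; GM_ReEarthLevel is the level logic Blueprint, apparently a game mode, for staged battles in the ReEarth level.
; On BeginPlay it caches actors tagged Battle_1 to Battle_4 as per-stage barrier lists and creates a player for the Trigger_1 level sequence.
; Tick polls StartStage1 and, while Wave is zero, plays that sequence and advances Wave to one.
; The barrier lists are only stored here, and only the first stage has logic.
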(event EventBeginPlay
  (Utilities|FlowControl|Sequence
    (:then_0
      (bind _outactors (Actor|GetAllActorswithTag "Battle_1"))
      (Variables|Default|SetBarrier_Stage1 _outactors))
    (:then_1
      (bind _outactors_2 (Actor|GetAllActorswithTag "Battle_2"))
      (Variables|Default|SetBarrier_Stage2 _outactors_2))
    (:then_2
      (bind _outactors_3 (Actor|GetAllActorswithTag "Battle_3"))
      (Variables|Default|SetBarrier_Stage3 _outactors_3))
    (:then_3
      (bind _outactors_4 (Actor|GetAllActorswithTag "Battle_4"))
      (Variables|Default|SetBarrier_Stage4 _outactors_4))
    (:then_4
      (bind _returnvalue (Sequencer|Player|CreateLevelSequencePlayer "/Game/AssetContents/SciFi_Hangars/Sequence/Trigger_1.Trigger_1"))
      (Variables|Default|SetTriggerSequence_1 _returnvalue))))

(event EventTick
  (params (DeltaSeconds :type Float%20%28single-precision%29))
  (if (Variables|Default|GetStart_Stage1)
    (switch int (Variables|Default|GetWave)
      (:0
        (Sequencer|Player|Play (Variables|Default|GetTriggerSequence_1) :!class /Script/MovieScene.MovieSceneSequencePlayer)
        (Variables|Default|SetWave 1)))))

(fn ConstructionScript)