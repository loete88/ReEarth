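; Game mode for the ReEarth level that gathers the barrier actors for four battle stages.
; On BeginPlay it finds actors by the Battle_1 to Battle_4 tags and caches each set in a matching BarrierStage variable.
; Tick checks a StartStage1 flag but the branch is empty, so the cached barriers are not yet used in this graph.
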(event EventBeginPlay
  (Utilities|FlowControl|Sequence
    (:then_0
      (bind _outactors (Actor|GetAllActorswithTag "Battle_1"))
      (Variables|Default|SetBarrier_Stage1 _outactors))
    (:then_1
      (bind _outactors_2 (Actor|GetAllActorswithTag "Battle_2"))
      (Variables|Default|SetBarrier_Stage2 _outactors_2))
    (:then_2
      (bind _outactors_3 (Actor|GetAllActorswithTag "Battle_3"))
      (Variables|Default|SetBarrier_Stage3 _outactors_3))
    (:then_3
      (bind _outactors_4 (Actor|GetAllActorswithTag "Battle_4"))
      (Variables|Default|SetBarrier_Stage4 _outactors_4))))

(event EventTick
  (params (DeltaSeconds :type Float%20%28single-precision%29))
  (if (Variables|Default|GetStart_Stage1)
    _))

(fn ConstructionScript)