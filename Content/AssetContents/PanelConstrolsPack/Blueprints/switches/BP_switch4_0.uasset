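; BP_switch4_0 is a switch prop from a control panel pack, posed entirely in the construction script with no active runtime logic.
; The script applies the MComponent material to slot 0 of both mesh components.
; Inside that same loop it adds a local roll to Component1, interpolated from SwitchPos remapped to a 0–1 alpha, so the rotation is applied once per mesh.
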(event EventBeginPlay)

(event Collision|EventActorBeginOverlap
  (params (OtherActor :type Actor%20Object%20Reference)))

(event EventTick
  (params (DeltaSeconds :type Float%20%28single-precision%29)))

(fn ConstructionScript
  ;[1 1 1] Set the material on each static mesh
  (Variables|Default|SetStaticMeshArray (Utilities|Array|MakeArray (Variables|Components|Getcomponent_1) (Variables|Default|Getcomponent_2)))
  (for _array_element (Variables|Default|GetStaticMeshArray)
    (Rendering|Material|SetMaterial _array_element 0 (Variables|Material|GetM_Component))
    (Transformation|AddLocalRotation (Variables|Components|Getcomponent_1) (Math|Rotator|MakeRotator (Math|Float|Lerp 5.0 -5.0 (* (+ (Variables|Float|Getswitch_pos) 1.0) 0.5)) 0.0 0.0) false false)))