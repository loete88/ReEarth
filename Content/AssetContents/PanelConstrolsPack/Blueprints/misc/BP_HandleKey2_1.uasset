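; BP_HandleKey2_1 is a panel-controls prop, apparently a two-key handle, configured entirely in its construction script.
; The script applies one shared material to three mesh components.
; KeyRot1 and KeyRot2 each map from a -1..1 range to a local yaw offset on their own mesh.
; These offsets are added inside the material loop, so they accumulate on every pass.
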(event EventBeginPlay)

(event Collision|EventActorBeginOverlap
  (params (OtherActor :type Actor%20Object%20Reference)))

(event EventTick
  (params (DeltaSeconds :type Float%20%28single-precision%29)))

(fn ConstructionScript
  ;[1 1 1] Set the material on each static mesh
  (Variables|Default|SetStaticMeshArray (Utilities|Array|MakeArray (Variables|Default|Getcomponent_2) (Variables|Default|Getcomponent_3) (Variables|Default|Getcomponent_4)))
  (for _array_element (Variables|Default|GetStaticMeshArray)
    (Rendering|Material|SetMaterial _array_element 0 (Variables|Material|GetM_Component))
    (Transformation|AddLocalRotation (Variables|Default|Getcomponent_3) (Math|Rotator|MakeRotator 0.0 0.0 (Math|Float|Lerp 6e+01 -6e+01 (* (+ (Variables|Float|Getkey_rot_1) 1.0) 0.5))) false false)
    (Transformation|AddLocalRotation (Variables|Default|Getcomponent_4) (Math|Rotator|MakeRotator 0.0 0.0 (Math|Float|Lerp 6e+01 -6e+01 (* (+ (Variables|Float|Getkey_rot_2) 1.0) 0.5))) false false)))