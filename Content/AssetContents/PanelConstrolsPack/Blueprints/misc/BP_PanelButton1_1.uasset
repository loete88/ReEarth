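; BP_PanelButton1_1 is a three-mesh control panel button prop, configured entirely in its construction script with no active event logic.
; A loop applies a shared material to each mesh, then overrides the first with glass.
; OpenClose drives the glass piece's roll and KeyRot, remapped from -1..1, drives the third mesh's yaw.
; These relative rotations sit inside the loop, so they accumulate on every iteration.
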(event EventBeginPlay)

(event Collision|EventActorBeginOverlap
  (params (OtherActor :type Actor%20Object%20Reference)))

(event EventTick
  (params (DeltaSeconds :type Float%20%28single-precision%29)))

(fn ConstructionScript
  ;[1 1 1] Set the material on each static mesh
  (Variables|Default|SetStaticMeshArray (Utilities|Array|MakeArray (Variables|Components|Getcomponent_1) (Variables|Default|Getcomponent_2) (Variables|Default|Getcomponent_3)))
  (for _array_element (Variables|Default|GetStaticMeshArray)
    (Rendering|Material|SetMaterial _array_element 0 (Variables|Material|GetM_Component))
    (Rendering|Material|SetMaterial (Variables|Components|Getcomponent_1) 0 (Variables|Material|GetM_Glass))
    (Transformation|AddLocalRotation (Variables|Components|Getcomponent_1) (Math|Rotator|MakeRotator (Math|Float|Lerp 0.0 35.0 (Variables|Float|GetOpen/Close)) 0.0 0.0) false false)
    (Transformation|AddLocalRotation (Variables|Default|Getcomponent_3) (Math|Rotator|MakeRotator 0.0 0.0 (Math|Float|Lerp 6e+01 -6e+01 (* (+ (Variables|Float|Getkey_rot) 1.0) 0.5))) false false)))