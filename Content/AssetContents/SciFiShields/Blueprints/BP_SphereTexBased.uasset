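; BP_SphereTexBased is a sci-fi shield sphere that plays a ring effect where a projectile hits it.
; When Sphere is hit by a BP_Projectile, it creates a dynamic material instance on StaticMeshComponent and passes it the impact point.
; A timeline then animates the HitRadius parameter, scaled by RingRadius, and applies RingHardness.
; Each hit creates the instance and restarts the single timeline.
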(event OnComponentHit(Sphere)
  (params (HitComponent :type Primitive%20Component%20Object%20Reference) (OtherActor :type Actor%20Object%20Reference) (OtherComp :type Primitive%20Component%20Object%20Reference) (NormalImpulse :type Vector :default "0, 0, 0") (Hit :type Hit%20Result%20Structure%20%28by%20ref%29))
  (Utilities|Casting|CastToBP_Projectile OtherActor)
  (bind _returnvalue (Rendering|Material|CreateDynamicMaterialInstance (Variables|Debug|GetStaticMeshComponent) 0 0 "None" :!class /Script/Engine.PrimitiveComponent))
  (Rendering|Material|SetVectorParameterValue _returnvalue "HitPosition" (Math|Conversions|ToLinearColor(Vector) (.ImpactPoint (Collision|BreakHitResult Hit))) :!class /Script/Engine.MaterialInstanceDynamic)
  (bind _radius (Timeline|Timeline_0 PlayFromStart)
    (:Update
      (Rendering|Material|SetScalarParameterValue _returnvalue "HitRadius" (* _radius (Variables|Default|GetRingRadius)) :!class /Script/Engine.MaterialInstanceDynamic)
      (Rendering|Material|SetScalarParameterValue _returnvalue "HitHardness" (Variables|Default|GetRingHardness) :!class /Script/Engine.MaterialInstanceDynamic))))

(fn ConstructionScript)