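; Sci-fi shield actor that shows a ripple reaction where a BP_Projectile hits its sphere collision.
; On hit, it passes the impact point to a dynamic material on the static mesh and spawns a particle burst oriented to the impact normal.
; A Radius timeline restarts on each hit, driving the material's ring radius, scaled by RingRadius, while RingHardness sets the hardness.
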(event OnComponentHit(Sphere)
  (params (HitComponent :type Primitive%20Component%20Object%20Reference) (OtherActor :type Actor%20Object%20Reference) (OtherComp :type Primitive%20Component%20Object%20Reference) (NormalImpulse :type Vector :default "0, 0, 0") (Hit :type Hit%20Result%20Structure%20%28by%20ref%29))
  (bind (_bblockinghit _binitialoverlap _time _distance _location _impactpoint _normal _impactnormal) (Collision|BreakHitResult Hit))
  ;[1 1 1] hIT
  (Utilities|Casting|CastToBP_Projectile OtherActor)
  (bind _returnvalue (Rendering|Material|CreateDynamicMaterialInstance (Variables|Debug|GetStaticMeshComponent) 0 0 "None" :!class /Script/Engine.PrimitiveComponent))
  (Rendering|Material|SetVectorParameterValue _returnvalue "HitPosition" (Math|Conversions|ToLinearColor(Vector) _impactpoint) :!class /Script/Engine.MaterialInstanceDynamic)
  (Effects|SpawnEmitteratLocation "/Game/AssetContents/SciFiShields/Particles/P_HitReaction.P_HitReaction" _impactpoint (Math|Rotator|MakeRotfromX _impactnormal))
  (bind _radius (Timeline|Radius PlayFromStart)
    (:Update
      (Rendering|Material|SetScalarParameterValue _returnvalue "HitPointRadius" (* _radius (Variables|Default|GetRingRadius)) :!class /Script/Engine.MaterialInstanceDynamic)
      (Rendering|Material|SetScalarParameterValue _returnvalue "HitHardness" (Variables|Default|GetRingHardness) :!class /Script/Engine.MaterialInstanceDynamic))))

(fn ConstructionScript)