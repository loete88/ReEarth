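; BP_EnemyType3 is an enemy character Blueprint that handles incoming damage and a ragdoll death state.
; AnyDamage prints a debug string and subtracts the damage from CurrentHP.
; While the remaining HP is still above zero, as the branch is wired, it ignores GameTraceChannel3 on the mesh, swaps in a dead physics asset, enables physics simulation and sets IsDead.
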(event Game|Damage|EventAnyDamage
  (params (Damage :type Float%20%28single-precision%29) (DamageType :type Damage%20Type%20Object%20Reference) (InstigatedBy :type Controller%20Object%20Reference) (DamageCauser :type Actor%20Object%20Reference))
  ;[1 1 1] AnyDamage
  (Development|PrintString "BP_EnemyType3")
  (Variables|Default|SetCurrentHP (- (Variables|Default|GetCurrentHP) Damage))
  (if (> (Variables|Default|GetCurrentHP) 0.0)
    (Collision|SetCollisionResponsetoChannel (Variables|Character|GetMesh) "ECC_GameTraceChannel3" "ECR_Ignore")
    (Components|SkinnedMesh|SetPhysicsAsset (Variables|Character|GetMesh) "/Game/AssetContents/ModularSciFiHeroesHP/Mesh/MeshForInternalAnimations/InternalAnim_PhysicsAsset_Dead.InternalAnim_PhysicsAsset_Dead" false)
    (Physics|SetSimulatePhysics (Variables|Character|GetMesh) true)
    (Variables|Default|SetIsDead true)))

(fn ConstructionScript)