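; BP_EnemyAI is an enemy AI controller that seeds the BB_Enemy blackboard and runs the BT_Enemy behavior tree.
; On BeginPlay it writes idle time, patrol radius and the pawn's starting location as home.
; SetAttackTarget stores a target and flags attack start unless one is already active, and IsAttackEnd sets the end flag and clears the start flag.
; An unconnected node for picking a random patrol point never runs.
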(event Custom|SetAttackTarget
  (params (NetAttackTarget :type BP%20Self%20Player%20Object%20Reference))
  ;[1 1 1] 코멘트
  (Development|PrintString "BP_EnemyAI_SetAttackTarget" false false)
  (if (not (ScalableFloat|GetValueasBool (AI|GetBlackboard 0) (Variables|Default|GetIsAttackStartKey)))
    (AI|Components|Blackboard|SetValueasBool (AI|GetBlackboard 0) (Variables|Default|GetIsAttackStartKey) true)
    (AI|Components|Blackboard|SetValueasObject (AI|GetBlackboard 0) (Variables|Default|GetAttackTargetkey) NetAttackTarget)))

(event Custom|IsAttackEnd
  (params (IsAttackEnd :type Boolean))
  ;[1 1 1] 코멘트
  (Development|PrintString "BP_EnemyAI_IsAttackEnd" false false)
  (AI|Components|Blackboard|SetValueasBool (AI|GetBlackboard 0) (Variables|Default|GetIsAttackEndKey) IsAttackEnd)
  (AI|Components|Blackboard|SetValueasBool (AI|GetBlackboard 0) (Variables|Default|GetIsAttackStartKey) false))

(event EventBeginPlay
  ;[1 1 1] BeginPlay
  (Utilities|FlowControl|Sequence
    (:then_0
      (Class|AIController|UseBlackboard "/Game/Enemy/AI/BB_Enemy.BB_Enemy")
      (AI|Components|Blackboard|SetValueasFloat (AI|GetBlackboard 0) (Variables|Default|GetIdleTimeKey) (Variables|Default|GetIdleTime))
      (AI|Components|Blackboard|SetValueasFloat (AI|GetBlackboard 0) (Variables|Default|GetPatrolRadiusKey) (Variables|Default|GetPatrolRadius))
      (AI|Components|Blackboard|SetValueasVector (AI|GetBlackboard 0) (Variables|Default|GetHomeLocKey) (Transformation|GetActorLocation (Pawn|GetControlledPawn))))
    (:then_1
      (AI|RunBehaviorTree "/Game/Enemy/AI/BT_Enemy.BT_Enemy"))))

(fn ConstructionScript)