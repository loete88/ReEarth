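; Enemy turret actor that turns toward and shoots at a FirstPersonCharacter it detects.
; Each PawnSensing sighting snaps the whole actor to face the character using a look-at rotation.
; It spawns a FirstPersonProjectile at ProjectileSpawnLocation and launches it with an impulse along the Cube's forward vector, scaled by ShootAmount.
; The SpawnProjectile flag and a Delay form a cooldown that limits the fire rate.
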(event OnSeePawn(PawnSensing)
  (params (Pawn :type Pawn%20Object%20Reference))
  (bind _asfirst_person_character (Utilities|Casting|CastToFirstPersonCharacter Pawn))
  (Utilities|FlowControl|Sequence
    (:then_0
      (Transformation|SetActorRotation (Math|Rotator|FindLookatRotation (Transformation|GetActorLocation) (Transformation|GetActorLocation _asfirst_person_character))))
    (:then_1
      (if (Variables|Default|GetSpawn%20Projectile)
        (bind _returnvalue (Game|SpawnActorfromClass "/Game/FirstPersonBP/Blueprints/FirstPersonProjectile.FirstPersonProjectile_C" (Transformation|GetWorldTransform (Variables|Default|GetProjectileSpawnLocation)) "Undefined" 0 0))
        (Physics|AddImpulse (Variables|/Game/FirstPersonBP/Blueprints/FirstPersonProjectile.FirstPersonProjectile_C|GetSphere _returnvalue) (* (Math|Vector|GetForwardVector (Variables|Default|GetCube)) (Variables|Default|GetShootAmount)) "None" false)
        (Variables|Default|SetSpawn%20Projectile false)
        (Utilities|FlowControl|Delay 1.5)
        (Variables|Default|SetSpawn%20Projectile true)))))

(fn ConstructionScript)