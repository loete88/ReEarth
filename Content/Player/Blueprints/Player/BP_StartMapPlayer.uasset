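; VR player for the start map, with two hands that grab and shoot, plus seat-mounted remote controllers.
; On BeginPlay it spawns both BP_Hand actors on VROrigin and the controllers on Seat sockets.
; Input actions forward grab and release to each hand, fire BP_Bullet from hand mesh transforms with sound and muzzle flash, or reset HMD orientation and position.
; SetJumpEnd and SetPlayerState are empty; GetDistanceSquare is a squared-distance helper.
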(event EventBeginPlay
  (bind _returnvalue (Math|Transform|MakeTransform "0, 0, 0"))
  (bind _self self)
  ;[1 1 1] VR Hand 생성
  (Utilities|FlowControl|Sequence
    (:then_0
      (bind _returnvalue_2 (Game|SpawnActorfromClass "/Game/Player/Blueprints/Controller/BP_Hand.BP_Hand_C" _returnvalue "AlwaysSpawn" _self "Left" 0))
      (Transformation|AttachComponentToComponent _returnvalue_2 (Variables|컴포넌트|GetVROrigin) "None" "SnapToTarget" "SnapToTarget" "KeepWorld" true)
      (Variables|Controller|SetLeftHand _returnvalue_2))
    (:then_1
      (bind _returnvalue_3 (Game|SpawnActorfromClass "/Game/Player/Blueprints/Controller/BP_Hand.BP_Hand_C" _returnvalue "AlwaysSpawn" _self "Right" 0))
      (Transformation|AttachComponentToComponent _returnvalue_3 (Variables|컴포넌트|GetVROrigin) "None" "SnapToTarget" "SnapToTarget" "KeepWorld" true)
      (Variables|Controller|SetRightHand _returnvalue_3))
    (:then_3
      ;[1 1 1] Controller 생성
      (bind _returnvalue_4 (Game|SpawnActorfromClass "/Game/Player/Blueprints/Controller/BP_Remote_Controller.BP_Remote_Controller_C" (Math|Transform|MakeTransform "0, 0, 0") "Undefined" self 0))
      (Transformation|AttachComponentToComponent (Variables|/Script/Engine.Actor|GetRootComponent _returnvalue_4) (Variables|Seat|GetSeat) "LeftControllerPosition" "SnapToTarget" "SnapToTarget" "KeepWorld" true)
      (bind _returnvalue_5 (Game|SpawnActorfromClass "/Game/Player/Blueprints/Controller/BP_ReMote_Controller_Right.BP_ReMote_Controller_Right_C" (Math|Transform|MakeTransform "0, 0, 0") "Undefined" self 0))
      (Transformation|AttachComponentToComponent (Variables|/Script/Engine.Actor|GetRootComponent _returnvalue_5) (Variables|Seat|GetSeat) "RightControllerPosition" "SnapToTarget" "SnapToTarget" "KeepWorld" true))))

(event Input|ActionEvents|InputActionLeftShot
  (params (Key :type Key%20Structure :default "None"))
  (:Pressed
    (Game|SpawnActorfromClass "/Game/Player/Blueprints/Bullet/BP_Bullet.BP_Bullet_C" (Transformation|GetWorldTransform (Variables|/Game/Player/Blueprints/Controller/BP_Hand.BP_Hand_C|GetHandMesh (Variables|Controller|GetLeftHand))) "Undefined" self 0)
    (Audio|PlaySoundatLocation "/Game/AssetContents/SciFiWeaponSoundFX/WeaponCue/RifleCue/Rifle8Mono_Cue.Rifle8Mono_Cue" "0, 0, 0" "0, 0, 0" 1.0 1.0 0.0 0 0 0)
    (Effects|SpawnEmitteratLocation "/Game/Player/Blueprints/Bullet/P_MuzzleFlash.P_MuzzleFlash" "0, 0, 0" "0, 0, 0" "2.000000,2.000000,2.000000")))

(event Input|ActionEvents|InputActionRightShot
  (params (Key :type Key%20Structure :default "None"))
  (:Pressed
    (Game|SpawnActorfromClass "/Game/Player/Blueprints/Bullet/BP_Bullet.BP_Bullet_C" (Transformation|GetWorldTransform (Variables|/Game/Player/Blueprints/Controller/BP_Hand.BP_Hand_C|GetHandMesh (Variables|Controller|GetRightHand))) "Undefined" self 0)
    (Audio|PlaySoundatLocation "/Game/AssetContents/SciFiWeaponSoundFX/WeaponCue/RifleCue/Rifle8Mono_Cue.Rifle8Mono_Cue" "0, 0, 0" "0, 0, 0" 1.0 1.0 0.0 0 0 0)
    (Effects|SpawnEmitteratLocation "/Game/Player/Blueprints/Bullet/P_MuzzleFlash.P_MuzzleFlash" "0, 0, 0" "0, 0, 0" "2.000000,2.000000,2.000000")))

(event Input|ActionEvents|InputActionVRReset
  (params (Key :type Key%20Structure :default "None"))
  (:Pressed
    (Class|HeadMountedDisplayFunctionLibrary|ResetOrientationandPosition 0.0 "OrientationAndPosition")))

(event Input|ActionEvents|InputActionGrabLeft
  (params (Key :type Key%20Structure :default "None"))
  (bind _lefthand (Variables|Controller|GetLeftHand))
  ;[1 1 1] VR Hand Event
  (:Pressed
    (Default|GrabActor _lefthand))
  (:Released
    (Default|ReleaseActor _lefthand)))

(event Input|ActionEvents|InputActionGrabRight
  (params (Key :type Key%20Structure :default "None"))
  (bind _righthand (Variables|Controller|GetRightHand))
  ;[1 1 1] VR Hand Event
  (:Pressed
    (Default|GrabActor _righthand))
  (:Released
    (Default|ReleaseActor _righthand)))

(fn ConstructionScript)

(fn SetJumpEnd)

(fn GetDistanceSquare
  (params (TargetLocation1 :type Vector) (TargetLocation2 :type Vector))
  (return (Math|Vector|VectorLengthSquared (- TargetLocation1 TargetLocation2))))

(fn SetPlayerState
  (params (NewPlayerState :type EM_PlayerState%20Enum :default "NewEnumerator0")))