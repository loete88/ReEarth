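; BP_Remote_Controller is a remote controller prop that the player picks up and docks back on the seat.
; Pickup disables mesh physics and snaps it to the given component's RemotePosition socket.
; Drop detaches it and snaps it to the player Seat's LeftControllerPosition socket, keeping physics off.
; Both events then switch BP_SelfPlayer's player state and left attack state.
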(event EventPickup
  (params (AttachTo :type Scene%20Component%20Object%20Reference))
  (Transformation|DetachFromActor "KeepWorld" "KeepWorld" "KeepWorld")
  (Physics|SetSimulatePhysics (Variables|Default|GetStaticMesh) false)
  (Transformation|AttachComponentToComponent (VehicleSound|GetRootComponent) AttachTo "RemotePosition" "SnapToTarget" "SnapToTarget" "KeepWorld" false)
  (bind _asbp_self_player (Utilities|Casting|CastToBP_SelfPlayer (Game|Player|GetPlayerPawn 0)))
  (Default|SetPlayerState _asbp_self_player "NewEnumerator0")
  (Variables|/Game/Player/Blueprints/Player/BP_SelfPlayer.BP_SelfPlayer_C|SetLeftAttackState _asbp_self_player "NewEnumerator0"))

(event EventDrop
  (Physics|SetSimulatePhysics (Variables|Default|GetStaticMesh) false)
  (Transformation|DetachFromActor "KeepWorld" "KeepWorld" "KeepWorld")
  (bind _asbp_self_player (Utilities|Casting|CastToBP_SelfPlayer (Game|Player|GetPlayerPawn 0)))
  (Transformation|AttachComponentToComponent (Variables|/Game/Player/Blueprints/Player/BP_SelfPlayer.BP_SelfPlayer_C|GetSeat _asbp_self_player) "LeftControllerPosition" "SnapToTarget" "SnapToTarget" "KeepWorld" true)
  (Default|SetPlayerState _asbp_self_player "NewEnumerator3")
  (Variables|/Game/Player/Blueprints/Player/BP_SelfPlayer.BP_SelfPlayer_C|SetLeftAttackState _asbp_self_player "NewEnumerator1"))

(fn ConstructionScript)